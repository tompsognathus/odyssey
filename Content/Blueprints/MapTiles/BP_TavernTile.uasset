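; BP_TavernTile is a map tile that switches between outside and inside tavern looks as the player enters and leaves.
; It applies the outside material to MapTile on BeginPlay.
; The Tavern component's overlap events swap that material to inside on entry and back to outside on exit.
; Entry only counts the player pawn's capsule component, while exit matches any component of the pawn.
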(event `self.ReceiveBeginPlay`
  (`parent.ReceiveBeginPlay`)
  (`PrimitiveComponent.SetMaterial` (`self.MapTile`) 0 "/Game/Materials/Maps/M_TavernOutside.M_TavernOutside"))

(event `self.tavern.OnComponentBeginOverlap`
  (params (OverlappedComponent :type "PrimitiveComponent Object Reference") (OtherActor :type "Actor Object Reference") (OtherComp :type "PrimitiveComponent Object Reference") (OtherBodyIndex :type Integer) (bFromSweep :type Boolean) (SweepResult :type "HitResult Structure (by ref)"))
  (if (== OtherComp (`self.GetComponentByClass` (`GameplayStatics.GetPlayerPawn` 0) "/Script/Engine.CapsuleComponent"))
    (`PrimitiveComponent.SetMaterial` (`self.MapTile`) 0 "/Game/Materials/Maps/M_TavernInside.M_TavernInside")))

(event `self.tavern.OnComponentEndOverlap`
  (params (OverlappedComponent :type "PrimitiveComponent Object Reference") (OtherActor :type "Actor Object Reference") (OtherComp :type "PrimitiveComponent Object Reference") (OtherBodyIndex :type Integer))
  (if (== OtherActor (`GameplayStatics.GetPlayerPawn` 0))
    (`PrimitiveComponent.SetMaterial` (`self.MapTile`) 0 "/Game/Materials/Maps/M_TavernOutside.M_TavernOutside")))

(fn `UserConstructionScript`
  (`parent.UserConstructionScript`))