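; Interactable treasure chest that highlights when in range and opens once on an interaction request.
; Interaction zone events toggle the highlight, and a request disables further interaction before running OpenTreasureLid.
; A timeline rotates the lid on roll toward OpenAngle with a creak sound.
; After a configurable delay from the start of opening, it activates the gold effect and plays coin spill and pickup sounds.
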(event `self.EnteredInteractionZone`
  (if (`self.IsInteractable`)
    (`Interactable.Highlight` true)))

(event `self.InteractRequest`
  (if (`self.IsInteractable`)
    (set `self.IsInteractable` false)
    (`Interactable.Highlight` false)
    (`self.OpenLid`)
    (`KismetSystemLibrary.Delay` (`self.GoldFXDelaySeconds`))
    (`ActorComponent.Activate` (`self.FX_Gold`) false)
    (`GameplayStatics.PlaySound2D` "/Game/Audio/SFX/coin_spill.coin_spill" 1.0 1.0 0.0 null null)
    (`GameplayStatics.PlaySound2D` "/Game/Audio/SFX/treasure_pickup.treasure_pickup" 1.0 1.0 0.0 null null)))

(event `OpenLid`
  (bind _openangle (`self.OpenAngle`))
  (`GameplayStatics.PlaySound2D` "/Game/Audio/SFX/treasure_chest_creak.treasure_chest_creak" 1.0 1.0 0.0 null null)
  (bind (_direction _lidrotation) (`Timeline|Timeline`)
    (:`Update`
      (`SceneComponent.K2_SetRelativeRotation` (`self.Lid`) (`KismetMathLibrary.MakeRotator` (* _lidrotation _openangle)) false false))
    (:`Finished`
      (`SceneComponent.K2_SetRelativeRotation` (`self.Lid`) (`KismetMathLibrary.MakeRotator` _openangle) false false))))

(event `self.LeftInteractionZone`
  (`Interactable.Highlight` false))

(fn `UserConstructionScript`)