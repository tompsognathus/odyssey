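; BP_LooseFloorboard is an interactable floorboard prop that signals its presence with an outline and a magic effect.
; On BeginPlay it registers its Cube mesh with the Highlighter, and entering or leaving the interaction zone toggles the highlight while IsInteractable is set.
; Separately, BoxCollision overlaps activate and deactivate FXMagic, with no check on the overlapping actor or interactable state.
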(event `self.ReceiveBeginPlay`
  (set `Highlighter.StaticMeshesToOutline` (`|MakeArray` (`self.Cube`)) (`self.Highlighter`)))

(event `self.EnteredInteractionZone`
  (if (`self.IsInteractable`)
    (`Interactable.Highlight` true)))

(event `self.LeftInteractionZone`
  (if (`self.IsInteractable`)
    (`Interactable.Highlight` false)))

(event `self.BoxCollision.OnComponentBeginOverlap`
  (params (OverlappedComponent :type "PrimitiveComponent Object Reference") (OtherActor :type "Actor Object Reference") (OtherComp :type "PrimitiveComponent Object Reference") (OtherBodyIndex :type Integer) (bFromSweep :type Boolean) (SweepResult :type "HitResult Structure (by ref)"))
  (`ActorComponent.Activate` (`self.FX_Magic`) true))

(event `self.BoxCollision.OnComponentEndOverlap`
  (params (OverlappedComponent :type "PrimitiveComponent Object Reference") (OtherActor :type "Actor Object Reference") (OtherComp :type "PrimitiveComponent Object Reference") (OtherBodyIndex :type Integer))
  (`ActorComponent.Deactivate` (`self.FX_Magic`)))

(fn `UserConstructionScript`)