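; Game mode that runs a Charisma conversational story session and connects it to the level's player, NPCs and entities.
; On BeginPlay it creates a playthrough and conversation, gathers entities, then starts the story and sets them live once connected.
; Messages run matching metadata function objects, give the speaking NPC text, audio and emotions, and turn other NPCs toward the speaker.
; Speech recognition results go to the player, and an end-story message closes their session.
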(event `OnMessageReceived`
  (params (MessageEvent :type "CharismaMessageEvent Structure (by ref)"))
  ;[1 1 1] Set Up Charisma Playthrough Handlers
  (`self.ParseMessage` MessageEvent))

(event `self.ReceiveBeginPlay`
  ;[1 1 1] Start Playthrough
  (bind (_playthrough _token _playthroughuuid _error) (`CreatePlaythroughToken.CreatePlaythroughToken` (`self.StoryId`) (`self.StoryVersion`) (`self.ApiKey`))
    (:`Success`
      (`|ExecutionSequence`
        (:`then_0`
          (set `self.Playthrough` _playthrough))
        (:`then_1`
          (bind _output_get (set `self.Token` _token)))
        (:`then_2`
          (set `self.Playthrough Uuid` _playthroughuuid))
        (:`then_3`
          (bind (_conversationuuid _error_2) (`CreateConversation.CreateConversation` _output_get)
            (:`Success`
              (set `self.Conversation Uuid` _conversationuuid)
              (`|ExecutionSequence`
                (:`then_0`
                  ;[1 1 1] Set Up Charisma Playthrough Handlers
                  (add `Playthrough.OnMessage` (`self.Playthrough`) (delegate `OnMessageReceived`)))
                (:`then_1`
                  (add `Playthrough.OnChangeConnectionState` (`self.Playthrough`) (delegate `OnConnectionStateChange`)))
                (:`then_2`
                  (`Playthrough.Connect` (`self.Playthrough`)))
                (:`then_3`
                  (`self.CollectAllCharismaEntities`))
                (:`then_4`
                  (add `Playthrough.OnSpeechRecognitionResult` (`self.Playthrough`) (delegate `OnSpeechResult`)))))
            (:`Failure`
              (`KismetSystemLibrary.PrintString` _error_2))))))
    (:`Failure`
      (`KismetSystemLibrary.PrintString` _error))))

(event `OnConnectionStateChange`
  (params (PreviousConnectionState :type "ECharismaPlaythroughConnectionState Enum" :default "Disconnected") (ConnectionState :type "ECharismaPlaythroughConnectionState Enum" :default "Disconnected"))
  ;[1 1 1] Set Up Charisma Playthrough Handlers
  (switch `ECharismaPlaythroughConnectionState` ConnectionState
    (:`Connected`
      (`Playthrough.Start` (`self.Playthrough`) (`self.Conversation Uuid`) 0 0 (`self.Start Graph Reference Id`) (`self.Speech Audio Format`))
      (`self.OnConversationStarted`)
      (`self.SetAllEntitiesLive`))))

(event `OnSpeechResult`
  (params (Transcript :type String) (IsFinal :type Boolean))
  ;[1 1 1] Set Up Charisma Playthrough Handlers
  (`/CharismaPlugNPlay/Blueprint/Player/BP_CharismaPlayerCharacter.SetSpeechResult` (`self.Player`) Transcript IsFinal))

(fn `ActorFullSend`
  (params (MessageToSend :type "CharismaMessageEvent Structure") (Actor :type "/CharismaPlugNPlay/Blueprint/Actors/BP_CharismaNPC_Female Object Reference"))
  (bind (_conversationuuid _type _message _endstory _taptocontinue _emotions) (break `CharismaMessageEvent` MessageToSend))
  (bind _charismapnpactor (`/CharismaPlugNPlay/Blueprint/Actors/BP_CharismaNPC_Female.CharismaPnPActor` Actor))
  (bind (_text _metadata _character _speech) (break `CharismaMessage` _message))
  ;[1 1 1] Full send - complete message parsing, including audio and speech
  (`/CharismaPlugNPlay/Blueprint/Actors/BP_CharismaNPC_Female.SetMessageBody` Actor _text)
  (`/CharismaPlugNPlay/Blueprint/Actors/BP_CharismaNPC_Female.SetSpeechData` Actor _speech)
  (if (> (`KismetArrayLibrary.Array_Length` _emotions) 0)
    ;[1 1 1] Apply all emotions present listed in Message if any are present
    (for _array_element _emotions
      (if (== (`.Name` (break `CharismaEmotion` _array_element)) (`CharismaEntityComponent.EntityId` _charismapnpactor))
        (`/CharismaPlugNPlay/Blueprint/Actors/BP_CharismaNPC_Female.Set ActiveEmotions` Actor _array_element))))
  (`/CharismaPlugNPlay/Blueprint/Actors/BP_CharismaNPC_Female.SetLookAtTarget` Actor (`self.Player`))
  (`CharismaPnPActorComponent.Resolve` _charismapnpactor))

(fn `ActorPartialSend`
  (params (MessageToSend :type "CharismaMessageEvent Structure") (Actor :type "/CharismaPlugNPlay/Blueprint/Actors/BP_CharismaNPC_Female Object Reference"))
  (for _array_element (`self.Actors`)
    (if (== (`CharismaEntityComponent.EntityId` (`/CharismaPlugNPlay/Blueprint/Actors/BP_CharismaNPC_Female.CharismaPnPActor` _array_element)) (`.Name` (break `CharismaCharacter` (`.Character` (break `CharismaMessage` (`.Message` (break `CharismaMessageEvent` MessageToSend)))))))
      (`/CharismaPlugNPlay/Blueprint/Actors/BP_CharismaNPC_Female.SetLookAtTarget` Actor _array_element)
      (`CharismaPnPActorComponent.Resolve` (`/CharismaPlugNPlay/Blueprint/Actors/BP_CharismaNPC_Female.CharismaPnPActor` Actor))
      (return))))

(fn `CollectAllCharismaEntities`
  (locals (ActorEntities :type "Array of CharismaPnPActorComponent Object Reference") (SimpleEntities :type "Array of CharismaEntityComponent Object Reference"))
  (`|ExecutionSequence`
    (:`then_0`
      (bind _returnvalue (`GameplayStatics.GetActorOfClass` "/CharismaPlugNPlay/Blueprint/Player/BP_CharismaPlayerCharacter.BP_CharismaPlayerCharacter_C"))
      (set `self.Player` _returnvalue))
    (:`then_1`
      (bind _outactors (`GameplayStatics.GetAllActorsOfClass` "/CharismaPlugNPlay/Blueprint/Actors/BP_CharismaNPC_Female.BP_CharismaNPC_Female_C"))
      (bind _output_get (set `self.Actors` _outactors))
      (for _array_element _output_get
        (`KismetArrayLibrary.Array_Add` (`local.ActorEntities`) (`self.GetComponentByClass` _array_element "/Script/CharismaPlugNPlay.CharismaPnPActorComponent"))))
    (:`then_2`
      (bind _outactors_2 (`GameplayStatics.GetAllActorsOfClass` "/CharismaPlugNPlay/Blueprint/Actors/Entities/BP_CharismaInteractableTemplate.BP_CharismaInteractableTemplate_C"))
      (for _array_element_2 _outactors_2
        (`KismetArrayLibrary.Array_Add` (`local.SimpleEntities`) (`self.GetComponentByClass` _array_element_2 "/Script/CharismaPlugNPlay.CharismaEntityComponent"))))
    (:`then_3`
      (`GameplayStatics.GetAllActorsOfClass` "/CharismaPlugNPlay/Blueprint/Actors/Entities/BP_CharismaMoveTo.BP_CharismaMoveTo_C")
      (for _array_element_3 _
        (`KismetArrayLibrary.Array_Add` (`local.SimpleEntities`) (`self.GetComponentByClass` _array_element_3 "/Script/CharismaPlugNPlay.CharismaEntityComponent"))))
    (:`then_4`
      (set `self.BaseEntities` (`local.SimpleEntities`)))
    (:`then_5`
      (for _array_element_4 (`self.MetadataClasses`)
        (bind _returnvalue_2 (`|GenericCreateObject` _array_element_4))
        (`KismetArrayLibrary.Array_Add` (`self.MetadataFunctions`) _returnvalue_2)
        (set `/CharismaPlugNPlay/Blueprint/Metadata/BP_MetadataFunction.PlaythroughEntities` (make `/CharismaPlugNPlay/Blueprint/BP_Struct_PlaythroughEntities` (`self.Player`) (`local.ActorEntities`) (`local.SimpleEntities`)) _returnvalue_2)))))

(fn `ParseMessage`
  (params (MessageEvent :type "CharismaMessageEvent Structure"))
  (locals (MessageBody :type "CharismaMessageEvent Structure"))
  (bind (_conversationuuid _type _message _endstory) (break `CharismaMessageEvent` MessageEvent))
  (bind (_text _metadata _character) (break `CharismaMessage` _message))
  (bind _output_get (set `local.MessageBody` MessageEvent))
  (`|ExecutionSequence`
    (:`then_0`
      ;[1 1 1] Try to parse metadata functions based on declared Functions
      (for _array_element (`self.MetadataFunctions`)
        (bind (_value _returnvalue) (`BlueprintMapLibrary.Map_Find` _metadata (`KismetStringLibrary.Conv_NameToString` (`/CharismaPlugNPlay/Blueprint/Metadata/BP_MetadataFunction.MetadataID` _array_element))))
        (if _returnvalue
          (`/CharismaPlugNPlay/Blueprint/Metadata/BP_MetadataFunction.Execute` _array_element _value))))
    (:`then_1`
      ;[1 1 1] Send Message to available Actors
      (if (not (`KismetStringLibrary.IsEmpty` (`.Name` (break `CharismaCharacter` _character))))
        (`self.TrySendToActors` _output_get)))
    (:`then_2`
      ;[1 1 1] Listen for EndStory message
      (if _endstory
        (`/CharismaPlugNPlay/Blueprint/Player/BP_CharismaPlayerCharacter.EndPlayerSession` (`self.Player`))))))

(fn `SetAllEntitiesLive`
  (for _array_element (`self.Actors`)
    (`CharismaEntityComponent.SetLive` (`/CharismaPlugNPlay/Blueprint/Actors/BP_CharismaNPC_Female.CharismaPnPActor` _array_element) true)
    (for _array_element_2 (`self.BaseEntities`)
      (`CharismaEntityComponent.SetLive` _array_element_2 true))))

(fn `TrySendToActors`
  (params (Message :type "CharismaMessageEvent Structure"))
  (for _array_element (`self.Actors`)
    (bind _returnvalue (`self.GetComponentByClass` _array_element "/Script/CharismaPlugNPlay.CharismaPnPActorComponent"))
    (if (`KismetSystemLibrary.IsValid` _returnvalue)
      (if (== (`CharismaEntityComponent.EntityId` _returnvalue) (`.Name` (break `CharismaCharacter` (`.Character` (break `CharismaMessage` (`.Message` (break `CharismaMessageEvent` Message)))))))
        (`self.ActorFullSend` Message _array_element)
        (else
          (`self.ActorPartialSend` Message _array_element))))))

(fn `UserConstructionScript`)