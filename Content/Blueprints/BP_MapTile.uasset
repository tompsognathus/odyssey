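; BP_MapTile is a map tile that switches the look of its ground when the player enters or leaves the tavern.
; Overlap events on the Tavern component check that the other actor is player 0's pawn.
; On begin overlap, GroundMap's first material slot gets the tavern interior material, and on end overlap it gets the exterior one.
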(event `self.tavern.OnComponentBeginOverlap`
  (params (OverlappedComponent :type "PrimitiveComponent Object Reference") (OtherActor :type "Actor Object Reference") (OtherComp :type "PrimitiveComponent Object Reference") (OtherBodyIndex :type Integer) (bFromSweep :type Boolean) (SweepResult :type "HitResult Structure (by ref)"))
  (if (== (`GameplayStatics.GetPlayerPawn` 0) OtherActor)
    (`PrimitiveComponent.SetMaterial` (`self.GroundMap`) 0 "/Game/Materials/Maps/M_TavernInside.M_TavernInside")))

(event `self.tavern.OnComponentEndOverlap`
  (params (OverlappedComponent :type "PrimitiveComponent Object Reference") (OtherActor :type "Actor Object Reference") (OtherComp :type "PrimitiveComponent Object Reference") (OtherBodyIndex :type Integer))
  (if (== (`GameplayStatics.GetPlayerPawn` 0) OtherActor)
    (`PrimitiveComponent.SetMaterial` (`self.GroundMap`) 0 "/Game/Materials/Maps/M_TavernOutside.M_TavernOutside")))

(fn `UserConstructionScript`)