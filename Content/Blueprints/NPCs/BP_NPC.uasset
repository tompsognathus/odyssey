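; BP_NPC is an NPC Blueprint that the player can interact with to start a dialogue.
; Entering the interaction zone turns on its highlight if IsInteractable is set, and leaving always turns it off.
; An interact request on an interactable NPC clears the highlight and calls StartDialogue with the first entry in Dialogues, passing itself as the only listed participant.
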(event `self.EnteredInteractionZone`
  (if (`self.IsInteractable`)
    (`Interactable.Highlight` true)))

(event `self.InteractRequest`
  (if (`self.IsInteractable`)
    (`Interactable.Highlight` false)
    (`self.StartDialogue` (`|GetArrayItem` (`self.Dialogues`)) (`|MakeArray` self :!type "Object Object Reference"))))

(event `self.LeftInteractionZone`
  (`Interactable.Highlight` false))

(fn `UserConstructionScript`)